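; Gold loot pickup that adds one gold to the TopDownCharacter that touches it, then destroys itself.
; Tick polls the static mesh's velocity and latches PickupEnabled once it is exactly zero, so the dropped loot is seen landing before it can be collected.
; Collection runs only on the sphere's begin-overlap event and is ignored until that flag is set.
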(event OnComponentBeginOverlap(Sphere)
  (params (OverlappedComponent :type Primitive%20Component%20Object%20Reference) (OtherActor :type Actor%20Object%20Reference) (OtherComp :type Primitive%20Component%20Object%20Reference) (OtherBodyIndex :type Integer) (bFromSweep :type Boolean) (SweepResult :type Hit%20Result%20Structure%20%28by%20ref%29))
  (if (Variables|Default|GetPickupEnabled)
    (bind _astop_down_character (Utilities|Casting|CastToTopDownCharacter OtherActor))
    (Math|Integer|IncrementInt (Variables|/Game/TopDownCPP/Blueprints/TopDownCharacter.TopDownCharacter_C|GetGold _astop_down_character)
      (:%20%20
        (Actor|DestroyActor)))))

(event EventTick
  (params (DeltaSeconds :type Float%20%28single-precision%29))
  ;[1 1 1] Can't pickup before it hits the ground, to see loot appear
  (if (not (Variables|Default|GetPickupEnabled))
    (Variables|Default|SetPickupEnabled (== (Math|Vector|VectorLength (Transformation|GetComponentVelocity (Variables|Default|GetStaticMesh))) 0.0))))

(fn ConstructionScript)