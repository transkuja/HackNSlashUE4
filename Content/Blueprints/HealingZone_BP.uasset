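; Healing zone actor that restores health to a TopDownCharacter standing inside its sphere.
; Sphere begin and end overlap events set and clear the stored player reference and an inside flag.
; While the flag is set, Tick uses a Delay as a throttle to heal about ten times a second.
; Each pulse passes negative damage to DamagePlayer and spawns a health pickup particle effect at the player's location.
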(event OnComponentBeginOverlap(Sphere)
  (params (OverlappedComponent :type Primitive%20Component%20Object%20Reference) (OtherActor :type Actor%20Object%20Reference) (OtherComp :type Primitive%20Component%20Object%20Reference) (OtherBodyIndex :type Integer) (bFromSweep :type Boolean) (SweepResult :type Hit%20Result%20Structure%20%28by%20ref%29))
  (bind _astop_down_character (Utilities|Casting|CastToTopDownCharacter OtherActor))
  (Variables|Default|SetPlayerIsIn true)
  (Variables|Default|SetPlayerRef _astop_down_character))

(event OnComponentEndOverlap(Sphere)
  (params (OverlappedComponent :type Primitive%20Component%20Object%20Reference) (OtherActor :type Actor%20Object%20Reference) (OtherComp :type Primitive%20Component%20Object%20Reference) (OtherBodyIndex :type Integer))
  (Utilities|Casting|CastToTopDownCharacter OtherActor)
  (Variables|Default|SetPlayerIsIn false)
  (Variables|Default|SetPlayerRef 0))

(event EventBeginPlay)

(event Collision|EventActorBeginOverlap
  (params (OtherActor :type Actor%20Object%20Reference)))

(event EventTick
  (params (DeltaSeconds :type Float%20%28single-precision%29))
  (bind _playerref (Variables|Default|GetPlayerRef))
  ;[1 1 1] Heal player
  (if (Variables|Default|GetPlayerIsIn)
    (Utilities|FlowControl|Delay 0.1)
    (Utilities|IsValid _playerref
      (:Is%20Valid
        (Default|DamagePlayer _playerref -1)
        (Effects|SpawnEmitteratLocation "/Game/InfinityBladeEffects/Effects/FX_Ability/Heal/P_Health_Pickup_01.P_Health_Pickup_01" (Transformation|GetActorLocation _playerref))))))

(fn ConstructionScript)