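; Healing well actor that can be switched off for a cooldown and then restores itself; the healing logic is not in this Blueprint.
; EnableWell toggles the mesh's visibility and query-only collision, setting Cooldown to InstanceCooldown when disabled and clearing it when enabled.
; Tick polls Cooldown and, while it is positive, runs a Delay of that length before re-enabling the well.
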(event EventBeginPlay)

(event Collision|EventActorBeginOverlap
  (params (OtherActor :type Actor%20Object%20Reference)))

(event EventTick
  (params (DeltaSeconds :type Float%20%28single-precision%29))
  (bind _cooldown (Variables|Default|GetCooldown))
  (if (> _cooldown 0)
    (Utilities|FlowControl|Delay (Math|Conversions|ToFloat(Integer) _cooldown))
    (CallFunction|EnableWell true)))

(fn ConstructionScript)

(fn EnableWell
  (params (Enable :type Boolean))
  (bind _staticmesh1 (Variables|Default|GetStaticMesh1))
  (Rendering|SetVisibility _staticmesh1 Enable false)
  (if Enable
    (Collision|SetCollisionEnabled _staticmesh1 "QueryOnly")
    (Variables|Default|SetCooldown 0)
    (else
      (Collision|SetCollisionEnabled _staticmesh1 "NoCollision")
      (Variables|Default|SetCooldown (Variables|Default|GetInstanceCooldown)))))