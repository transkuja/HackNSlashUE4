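; HUD Blueprint that creates the permanent on-screen UI and a hidden inventory widget at BeginPlay.
; It binds event dispatchers for closing and opening, toggling the inventory and slot visibility and switching between UI-only and game-and-UI input modes.
; It also seeds the first twelve slots with test items: a helmet, then alternating shields and swords.
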(event Custom|CloseEvent
  ;[0.3904 1 0.6632] Listen event dispatcher created in Inventory
  ;[1 0.9225 0.3229] Display/Hide Inventory widget
  (Widget|SetVisibility (Variables|Default|GetInventory) "Hidden")
  (Input|SetInputModeGameandUI (Game|GetPlayerController 0) 0 "DoNotLock" false)
  (for _array_element (Variables|/Game/Inventory/Widgets/Inventory_UI.Inventory_UI_C|GetItemSlots (Variables|Default|GetInventory))
    (Widget|SetVisibility _array_element "Hidden")
    (Class|WidgetBlueprintLibrary|SetFocustoGameViewport)))

(event Custom|OpenEvent
  (bind _inventory (Variables|Default|GetInventory))
  ;[0.3904 1 0.6632] Listen event dispatcher created in Inventory
  ;[1 0.9225 0.3229] Display/Hide Inventory widget
  (Widget|SetVisibility (Variables|Default|GetInventory) "Visible")
  (Input|SetInputModeUIOnly (Game|GetPlayerController 0) _inventory "DoNotLock")
  (for _array_element (Variables|/Game/Inventory/Widgets/Inventory_UI.Inventory_UI_C|GetItemSlots _inventory)
    (Widget|SetVisibility _array_element "Visible")))

(event EventBeginPlay
  ;[1 0.3851 0.405] Create and reference Inventory Widget
  (bind _returnvalue (UserInterface|CreateWidget "/Game/Blueprints/UI/PermanentUI_BP.PermanentUI_BP_C"))
  (bind _output_get (Variables|Default|SetPermanentUI _returnvalue))
  (UserInterface|Viewport|AddtoViewport _output_get 0)
  (bind _returnvalue_2 (UserInterface|CreateWidget "/Game/Inventory/Widgets/Inventory_UI.Inventory_UI_C"))
  (bind _output_get_2 (Variables|Default|SetInventory _returnvalue_2))
  (UserInterface|Viewport|AddtoViewport _output_get_2 0)
  (Widget|SetVisibility _output_get_2 "Hidden")
  ;[0.3904 1 0.6632] Listen event dispatcher created in Inventory
  (EventDispatchers|BindEventtoCloseED (Variables|Default|GetInventory) (delegate Custom|CloseEvent))
  (EventDispatchers|BindEventtoOpenInventoryED (delegate Custom|OpenEvent))
  ;[0 0.1472 1] Add Some items
  (for _index (range 0 11)
    (bind _returnvalue_3 (UserInterface|CreateWidget "/Game/Inventory/Widgets/ItemWidget_UI.ItemWidget_UI_C" (Game|GetPlayerController 0)))
    (if (== _index 0)
      (Default|CreateHelmet _returnvalue_3)
      (elif (== (Math|Integer|%(Integer) _index 2) 0)
        (Default|CreateSword _returnvalue_3)
        (else
          (Default|CreateShield _returnvalue_3))))
    (Default|AddItemtoThisSlot (Utilities|Array|Get(acopy) (Variables|/Game/Inventory/Widgets/Inventory_UI.Inventory_UI_C|GetItemSlots (Variables|Default|GetInventory)) _index) _returnvalue_3)))

(fn ConstructionScript)