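; AiStatsComponent is an actor component holding AI combat stats: strength, health, dexterity, experience reward or value, and attack and chase ranges.
; BeginPlay seeds these stats with hardcoded defaults, applying dexterity through UpdateDexterity.
; UpdateDexterity adds to Dexterity and, only when the owner is an OldLady_BP, scales its CharacterMovement max walk speed from the new total.
; UpdateEndurance is an empty stub.
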(event EventBeginPlay
  (Variables|Default|SetStrength 25)
  (Variables|Default|SetHealth 70)
  (Variables|Default|SetMaxHealth 70)
  (Variables|Default|SetExp 20)
  (CallFunction|UpdateDexterity 80)
  (Variables|Default|SetRange 2e+02)
  (Variables|Default|SetRunToPlayerRange 4e+02))

(fn UpdateDexterity
  (params (Dexterity%20to%20add :type Integer))
  (bind _returnvalue (Components|GetOwner))
  (bind _output_get (Variables|Default|SetDexterity (+ (Variables|Default|GetDexterity) Dexterity%20to%20add)))
  (Utilities|Casting|CastToOldLady_BP _returnvalue)
  (Variables|/Script/Engine.CharacterMovementComponent|SetMaxWalkSpeed (Actor|GetComponentbyClass _returnvalue "/Script/Engine.CharacterMovementComponent") (+ 6e+02 (Math|Conversions|ToFloat(Integer) (* _output_get 3)))))

(fn UpdateEndurance)