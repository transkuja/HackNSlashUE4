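; Enemy old lady character that chases the player, attacks in range and awards experience and a kill when defeated.
; Tick compares player distance to AiStatsComponent ranges to drive movement, facing and the anim Blueprint's attack flag, with Dexterity passed for attack speed.
; Damage events lower clamped health and update the HealthBar widget.
; Death hides the bar, ragdolls the body with an impulse up and away from the player, then destroys it after a delay.
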(event Custom|ReceiveDamage
  (params (DamagedActor :type Actor%20Object%20Reference) (Damage :type Float%20%28single-precision%29) (DamageType :type Damage%20Type%20Object%20Reference) (InstigatedBy :type Controller%20Object%20Reference) (DamageCauser :type Actor%20Object%20Reference))
  ;[1 0 0.7175] Override take damage event
  (CallFunction|ReceiveDmg (.AsOld%20Lady%20BP (Utilities|Casting|CastToOldLady_BP DamagedActor)) (Math|Float|Round Damage)))

(event Custom|KillGranny
  (bind _returnvalue (Game|GetPlayerCharacter 0))
  (bind _astop_down_character (Utilities|Casting|CastToTopDownCharacter _returnvalue))
  ;[1 1 1] On death event
  ;;[0.1337 0.6172 0.81] Freeze anim
  (Variables|Default|SetisDead true)
  (Variables|/Game/Character/Enemies/OldLadyAnim_BP.OldLadyAnim_BP_C|SetisAttacking (Variables|Default|GetAnimInstance) false)
  (Default|UpdateExperience _astop_down_character (Variables|/Game/Blueprints/AiStatsComponent.AiStatsComponent_C|GetExp (Variables|Default|GetAiStatsComponent)))
  (Default|UpdateKills _astop_down_character)
  (Widget|SetVisibility (UserInterface|GetUserWidgetObject (Variables|Default|GetHealthBar)) "Hidden")
  (CallFunction|EjectGranny)
  (Utilities|FlowControl|Delay 3.0)
  (Actor|DestroyActor))

(event EventBeginPlay
  (bind _aistatscomponent (Variables|Default|GetAiStatsComponent))
  (bind _healthbar (Variables|Default|GetHealthBar))
  (bind _returnvalue (UserInterface|GetUserWidgetObject _healthbar))
  (bind _ashealth_bar (Utilities|Casting|CastToHealthBar _returnvalue))
  ;[1 1 1] Init BP
  ;[1 0 0.7175] Override take damage event
  (EventDispatchers|BindEventtoOnTakeAnyDamage (delegate Custom|ReceiveDamage))
  (bind _asold_lady_anim_bp (Utilities|Casting|CastToOldLadyAnim_BP (Components|SkeletalMesh|GetAnimInstance (Variables|Character|GetMesh))))
  (bind _output_get (Variables|Default|SetAnimInstance _asold_lady_anim_bp))
  ;[1 1 1] Send dexterity to anim BP for attack speed
  (Variables|/Game/Character/Enemies/OldLadyAnim_BP.OldLadyAnim_BP_C|SetDexterity _output_get (Math|Conversions|ToFloat(Integer) (Variables|/Game/Blueprints/AiStatsComponent.AiStatsComponent_C|GetDexterity (Variables|Default|GetAiStatsComponent))))
  ;[1 1 1] Init health
  (Variables|/Game/Blueprints/UI/HealthBar.HealthBar_C|SetHealth _ashealth_bar (Variables|/Game/Blueprints/AiStatsComponent.AiStatsComponent_C|GetHealth _aistatscomponent))
  (Variables|/Game/Blueprints/UI/HealthBar.HealthBar_C|SetMaxHealth _ashealth_bar (Variables|/Game/Blueprints/AiStatsComponent.AiStatsComponent_C|GetMaxHealth _aistatscomponent)))

(event Collision|EventActorBeginOverlap
  (params (OtherActor :type Actor%20Object%20Reference)))

(event EventTick
  (params (DeltaSeconds :type Float%20%28single-precision%29))
  (bind _returnvalue (Game|GetPlayerCharacter 0))
  (bind _animinstance (Variables|Default|GetAnimInstance))
  (bind _returnvalue_2 (Transformation|GetDistanceTo _returnvalue))
  (if (not (Variables|Default|GetisDead))
    ;[1 1 1] Look at player if is attacking
    (if (Variables|/Game/Character/Enemies/OldLadyAnim_BP.OldLadyAnim_BP_C|GetisAttacking (Variables|Default|GetAnimInstance))
      (CallFunction|LookatPlayer))
    ;[1 1 1] Play/Stop attack anim if the player is close enough
    (if (< _returnvalue_2 (Variables|/Game/Blueprints/AiStatsComponent.AiStatsComponent_C|GetRange (Variables|Default|GetAiStatsComponent)))
      (if (not (Variables|/Game/Character/Enemies/OldLadyAnim_BP.OldLadyAnim_BP_C|GetisAttacking (Variables|Default|GetAnimInstance)))
        (Variables|/Game/Character/Enemies/OldLadyAnim_BP.OldLadyAnim_BP_C|SetisAttacking _animinstance true))
      (else
        (if (Variables|/Game/Character/Enemies/OldLadyAnim_BP.OldLadyAnim_BP_C|GetisAttacking (Variables|Default|GetAnimInstance))
          (Variables|/Game/Character/Enemies/OldLadyAnim_BP.OldLadyAnim_BP_C|SetisAttacking _animinstance false))
        ;[1 1 1] Follow player if in range
        (if (< _returnvalue_2 (Variables|/Game/Blueprints/AiStatsComponent.AiStatsComponent_C|GetRunToPlayerRange (Variables|Default|GetAiStatsComponent)))
          (CallFunction|LookatPlayer)
          (AI|Navigation|SimpleMovetoLocation (Pawn|GetController) (Transformation|GetActorLocation (Game|GetPlayerCharacter 0))))))))

(fn ConstructionScript)

(fn LookatPlayer
  ;[1 1 1] Look at player when attacking
  (Transformation|SetWorldRotation (VehicleSound|GetRootComponent) (Math|Rotator|MakeRotator 0.0 0.0 (.yaw (Math|Rotator|FindLookatRotation (Transformation|GetActorLocation) (Transformation|GetActorLocation (Game|GetPlayerCharacter 0))))) false false))

(fn ReceiveDmg
  (params (Damage%20to%20add :type Integer))
  (bind _aistatscomponent (Variables|Default|GetAiStatsComponent))
  (if (not (Variables|Default|GetisDead))
    (bind _output_get (Variables|/Game/Blueprints/AiStatsComponent.AiStatsComponent_C|SetHealth _aistatscomponent (Math|Integer|Clamp(Integer) (- (Variables|/Game/Blueprints/AiStatsComponent.AiStatsComponent_C|GetHealth _aistatscomponent) Damage%20to%20add) 0 (Variables|/Game/Blueprints/AiStatsComponent.AiStatsComponent_C|GetMaxHealth _aistatscomponent))))
    (Variables|/Game/Blueprints/UI/HealthBar.HealthBar_C|SetHealth (.AsHealth%20Bar (Utilities|Casting|CastToHealthBar (UserInterface|GetUserWidgetObject (Variables|Default|GetHealthBar)))) _output_get)
    (if (== (Math|Integer|Clamp(Integer) (- (Variables|/Game/Blueprints/AiStatsComponent.AiStatsComponent_C|GetHealth _aistatscomponent) Damage%20to%20add) 0 (Variables|/Game/Blueprints/AiStatsComponent.AiStatsComponent_C|GetMaxHealth _aistatscomponent)) 0)
      (CallFunction|KillGranny))))

(fn EjectGranny
  (bind _mesh (Variables|Character|GetMesh))
  ;[1 1 1] Enable physics
  (Collision|SetCollisionEnabled _mesh "QueryAndPhysics")
  (Class|SkeletalMeshComponent|SetAllBodiesSimulatePhysics _mesh true)
  (Class|SkeletalMeshComponent|SetAllBodiesPhysicsBlendWeight (Variables|Character|GetMesh) 1.0 false)
  (Physics|SetSimulatePhysics (Variables|Collision|GetCapsuleComponent) true)
  (Class|SkeletalMeshComponent|AddImpulsetoAllBodiesBelow (Variables|Character|GetMesh) (* (+ (Math|Vector|Normalize (- (Transformation|GetActorLocation) (Transformation|GetActorLocation (Game|GetPlayerCharacter 0)))) "0,0.000000,1.000000") 8e+03) "None" false true))