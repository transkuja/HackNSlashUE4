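; CustomController_BP is a player controller that handles mouse and inventory input for a top-down character.
; It enables click and mouse-over events, and the Inventory action asks HUD_BP to open the inventory.
; A right-click trace under the cursor sends the player toward a hit OldLady_BP and stores it as TopDownCharacter's ClickTarget, clearing the target otherwise.
; A left click also clears ClickTarget.
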(event EventBeginPlay
  (Variables|Default|SetbEnableClickEvents true)
  (Variables|Default|SetbEnableMouseOverEvents true))

(event EventTick
  (params (DeltaSeconds :type Float%20%28single-precision%29)))

(event Input|ActionEvents|InputActionInventory
  (params (Key :type Key%20Structure :default "AnyKey"))
  (:Pressed
    (Default|CallOpenInventoryED (.AsHUD%20BP (Utilities|Casting|CastToHUD_BP (HUD|GetHUD))))))

(event Input|MouseEvents|RightMouseButton
  (params (Key :type Key%20Structure :default "AnyKey"))
  (bind _returnvalue (Game|GetPlayerCharacter 0))
  (bind _astop_down_character (Utilities|Casting|CastToTopDownCharacter _returnvalue))
  (:Pressed
    ;[1 1 1] Move to clicked target if valid or reset it
    (bind _asold_lady_bp (Utilities|Casting|CastToOldLady_BP (.HitActor (Collision|BreakHitResult (.HitResult (Game|Player|GetHitResultUnderCursorbyChannel "TraceTypeQuery1" true)))))
      (:then
        (AI|Navigation|SimpleMovetoActor self _asold_lady_bp)
        (Variables|/Game/TopDownCPP/Blueprints/TopDownCharacter.TopDownCharacter_C|SetClickTarget _astop_down_character _asold_lady_bp))
      (:CastFailed
        (Variables|/Game/TopDownCPP/Blueprints/TopDownCharacter.TopDownCharacter_C|SetClickTarget _astop_down_character 0)))))

(event Input|MouseEvents|LeftMouseButton
  (params (Key :type Key%20Structure :default "AnyKey"))
  ;[1 1 1] Reset clicked target on move
  (:Pressed
    (Variables|/Game/TopDownCPP/Blueprints/TopDownCharacter.TopDownCharacter_C|SetClickTarget (.AsTop%20Down%20Character (Utilities|Casting|CastToTopDownCharacter (Game|GetPlayerCharacter 0))) 0)))

(fn ConstructionScript)