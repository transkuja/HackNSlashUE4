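; Spawner actor that creates OldLadyBP enemies at its own transform while Enabled, paced by a Delay on Tick.
; Each spawn, depending on OnSpawnBehavior, is sent by simple AI move toward the player character or the HeadTo location.
; DifficultyUpdate scales an actor's AiStatsComponent dexterity, health, strength and Exp by a quadratic Difficulty ratio, but the spawn flow never calls it.
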(event EventBeginPlay)

(event EventTick
  (params (DeltaSeconds :type Float%20%28single-precision%29))
  ;[1 1 1] Spawn with a delay
  (if (Variables|Default|GetEnabled)
    (Utilities|FlowControl|Delay (Variables|Default|GetSpawnTick))
    (bind _returnvalue (Game|SpawnActorfromClass (Variables|SpawnOptions|GetOldLadyBP) (Transformation|GetActorTransform) "Undefined" 0 0))
    (switch Utilities|FlowControl|Switch|SwitchonSpawnState (Variables|Default|GetOnSpawnBehavior)
      (:NewEnumerator1
        (AI|Navigation|SimpleMovetoActor (Pawn|GetController (Variables|/Script/Engine.Actor|GetInstigator _returnvalue)) (Game|GetPlayerCharacter 0)))
      (:NewEnumerator2
        (AI|Navigation|SimpleMovetoLocation (Pawn|GetController (Variables|/Script/Engine.Actor|GetInstigator _returnvalue)) (Transformation|GetWorldLocation (Variables|Default|GetHeadTo)))))))

(fn ConstructionScript)

(fn DifficultyUpdate
  (params (Actor :type Actor%20Object%20Reference))
  (bind _returnvalue (Actor|GetComponentbyClass Actor "/Game/Blueprints/AiStatsComponent.AiStatsComponent_C"))
  (bind _difficulty_multiplier (CallFunction|GetDifficultyRatio (Variables|Default|GetDifficulty)))
  (LocalVariables|SetDifficultyRatio _difficulty_multiplier)
  (Default|UpdateDexterity _returnvalue (Math|Float|Ceil (* (Math|Conversions|ToFloat(Integer) (Variables|/Game/Blueprints/AiStatsComponent.AiStatsComponent_C|GetDexterity _returnvalue)) _difficulty_multiplier)))
  (Variables|/Game/Blueprints/AiStatsComponent.AiStatsComponent_C|SetMaxHealth _returnvalue (Math|Float|Ceil (* (Math|Conversions|ToFloat(Integer) (Variables|/Game/Blueprints/AiStatsComponent.AiStatsComponent_C|GetMaxHealth _returnvalue)) (LocalVariables|GetDifficultyRatio))))
  (Variables|/Game/Blueprints/AiStatsComponent.AiStatsComponent_C|SetHealth _returnvalue (Math|Float|Ceil (* (Math|Conversions|ToFloat(Integer) (Variables|/Game/Blueprints/AiStatsComponent.AiStatsComponent_C|GetHealth _returnvalue)) (LocalVariables|GetDifficultyRatio))))
  (Variables|/Game/Blueprints/AiStatsComponent.AiStatsComponent_C|SetStrength _returnvalue (Math|Float|Ceil (* (Math|Conversions|ToFloat(Integer) (Variables|/Game/Blueprints/AiStatsComponent.AiStatsComponent_C|GetStrength _returnvalue)) (LocalVariables|GetDifficultyRatio))))
  (Variables|/Game/Blueprints/AiStatsComponent.AiStatsComponent_C|SetExp _returnvalue (Math|Float|Ceil (* (Math|Conversions|ToFloat(Integer) (Variables|/Game/Blueprints/AiStatsComponent.AiStatsComponent_C|GetExp _returnvalue)) (LocalVariables|GetDifficultyRatio)))))

(fn GetDifficultyRatio
  (params (Current%20Difficulty :type Integer))
  (return (+ (* (* Current%20Difficulty Current%20Difficulty) 0.1) 1.0)))