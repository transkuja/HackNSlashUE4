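; Player controller for a top-down click game that enables mouse clicks and hover events and handles inventory and interaction input.
; While the player is alive, the Inventory action opens the HUD inventory and right click traces under the cursor.
; Hits on OldLady, WaveHandler, PNJ or HealingWell actors become the character's ClickTarget and are walked to via SimpleMoveToActor.
; Other hits clear the target and pick up any Item_BP, while left click just clears the target.
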(event EventBeginPlay
  ;[1 1 1] Enable mouse
  (Variables|Default|SetbEnableClickEvents true)
  (Variables|Default|SetbEnableMouseOverEvents true))

(event Input|ActionEvents|InputActionInventory
  (params (Key :type Key%20Structure :default "AnyKey"))
  ;[1 1 1] Inventory input
  (:Pressed
    (if (not (Variables|/Game/TopDownCPP/Blueprints/TopDownCharacter.TopDownCharacter_C|GetisPlayerDead (.AsTop%20Down%20Character (Utilities|Casting|CastToTopDownCharacter (Game|GetPlayerCharacter 0)))))
      (Default|CallOpenInventoryED (.AsHUD%20BP (Utilities|Casting|CastToHUD_BP (HUD|GetHUD)))))))

(event Input|MouseEvents|RightMouseButton
  (params (Key :type Key%20Structure :default "AnyKey"))
  (bind _hitresult (Game|Player|GetHitResultUnderCursorbyChannel "TraceTypeQuery1" true))
  (bind _returnvalue (Game|GetPlayerCharacter 0))
  (bind _hitactor (Collision|BreakHitResult _hitresult))
  (bind _astop_down_character (Utilities|Casting|CastToTopDownCharacter _returnvalue))
  (:Pressed
    (if (not (Variables|/Game/TopDownCPP/Blueprints/TopDownCharacter.TopDownCharacter_C|GetisPlayerDead (.AsTop%20Down%20Character (Utilities|Casting|CastToTopDownCharacter (Game|GetPlayerCharacter 0)))))
      ;[1 1 1] Move to clicked target if valid
      (if (Math|Boolean|ORBoolean (.bSuccess (Utilities|Casting|CastToOldLady_BP _hitactor)) (.bSuccess (Utilities|Casting|CastToWaveHandler_BP _hitactor)) (.bSuccess (Utilities|Casting|CastToPNJ_BP _hitactor)) (.bSuccess (Utilities|Casting|CastToHealingWell_BP _hitactor)))
        (AI|Navigation|SimpleMovetoActor self _hitactor)
        (Variables|/Game/TopDownCPP/Blueprints/TopDownCharacter.TopDownCharacter_C|SetClickTarget _astop_down_character _hitactor)
        (else
          (Variables|/Game/TopDownCPP/Blueprints/TopDownCharacter.TopDownCharacter_C|SetClickTarget _astop_down_character 0)
          ;[1 1 1] Pickup item on right click
          (bind _asitem_bp (Utilities|Casting|CastToItem_BP _hitactor))
          (Default|PickupItem _asitem_bp))))))

(event Input|MouseEvents|LeftMouseButton
  (params (Key :type Key%20Structure :default "AnyKey"))
  ;[1 1 1] Reset clicked target on move
  (:Pressed
    (Variables|/Game/TopDownCPP/Blueprints/TopDownCharacter.TopDownCharacter_C|SetClickTarget (.AsTop%20Down%20Character (Utilities|Casting|CastToTopDownCharacter (Game|GetPlayerCharacter 0))) 0)))

(fn ConstructionScript)