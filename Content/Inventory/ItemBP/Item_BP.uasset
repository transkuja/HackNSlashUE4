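; Item_BP is a clickable world item that can be picked up into the HUD inventory and equipped for stat bonuses.
; Clicking an unequipped item creates a helmet, shield or sword widget from its type flags, fills the first empty slot and destroys the actor.
; EquipItem and RemoveItem add or subtract StatsComponent Strength, Endurance and Dexterity on the TopDownCharacter.
; Overlapping an OldLady_BP ragdolls her with an impulse, marked for removal.
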(event OnClicked(SkeletalMesh)
  (params (TouchedComponent :type Primitive%20Component%20Object%20Reference) (ButtonPressed :type Key%20Structure :default "AnyKey"))
  (bind _returnvalue (Game|GetPlayerController 0))
  (bind _returnvalue_2 (HUD|GetHUD _returnvalue))
  (bind _ashud_bp (Utilities|Casting|CastToHUD_BP _returnvalue_2))
  (bind _inventory (Variables|/Game/Blueprints/HUD_BP.HUD_BP_C|GetInventory _ashud_bp))
  (bind _itemslots (Variables|/Game/Inventory/Widgets/Inventory_UI.Inventory_UI_C|GetItemSlots _inventory))
  ;[1 1 1] Pickup item
  ;;[1 0.2479 0.9179] Check if the item is on the ground
  (if (not (Variables|Default|GetisEquipped))
    (bind _index (Utilities|FlowControl|ForLoopwithBreak 0 (Utilities|Array|Length _itemslots) :!label _label)
      (:LoopBody
        (Utilities|IsValid (Variables|/Game/Inventory/Widgets/ItemSlot_UI.ItemSlot_UI_C|GetItemInThisSlot (Utilities|Array|Get(acopy) _itemslots _index))
          (:Is%20Not%20Valid
            (bind _returnvalue_3 (UserInterface|CreateWidget "/Game/Inventory/Widgets/ItemWidget_UI.ItemWidget_UI_C"))
            (if (Variables|Default|GetisHelmet)
              (Default|CreateHelmet _returnvalue_3)
              (Default|AddItemtoThisSlot (Utilities|Array|Get(acopy) _itemslots _index) _returnvalue_3 :!label _label_2)
              (Actor|DestroyActor)
              (goto _label Break)
              (elif (Variables|Default|GetisLeftHand)
                (Default|CreateShield _returnvalue_3)
                (goto _label_2)
                (elif (Variables|Default|GetisRightHand)
                  (Default|CreateSword _returnvalue_3)
                  (goto _label_2))))))))))

(event OnComponentBeginOverlap(SkeletalMesh)
  (params (OverlappedComponent :type Primitive%20Component%20Object%20Reference) (OtherActor :type Actor%20Object%20Reference) (OtherComp :type Primitive%20Component%20Object%20Reference) (OtherBodyIndex :type Integer) (bFromSweep :type Boolean) (SweepResult :type Hit%20Result%20Structure%20%28by%20ref%29))
  ;[1 0 0.956] Remove this shit
  (bind _asold_lady_bp (Utilities|Casting|CastToOldLady_BP OtherActor))
  (Collision|SetCollisionEnabled (Variables|/Game/Character/Enemies/OldLady_BP.OldLady_BP_C|GetSkeletalMesh _asold_lady_bp) "QueryAndPhysics")
  (Class|SkeletalMeshComponent|SetAllBodiesSimulatePhysics (Variables|/Game/Character/Enemies/OldLady_BP.OldLady_BP_C|GetSkeletalMesh _asold_lady_bp) true)
  (Class|SkeletalMeshComponent|SetAllBodiesPhysicsBlendWeight (Variables|/Game/Character/Enemies/OldLady_BP.OldLady_BP_C|GetSkeletalMesh _asold_lady_bp) 1.0 false)
  (Physics|SetSimulatePhysics (Variables|/Game/Character/Enemies/OldLady_BP.OldLady_BP_C|GetSkeletalMesh _asold_lady_bp) true)
  (Physics|AddImpulse (Variables|/Game/Character/Enemies/OldLady_BP.OldLady_BP_C|GetSkeletalMesh _asold_lady_bp) (* (+ (* (.ImpactNormal (Collision|BreakHitResult SweepResult)) -1.0) "0,1.000000, 0") 2.5e+03) "None" false))

(event EventBeginPlay)

(event Collision|EventActorBeginOverlap
  (params (OtherActor :type Actor%20Object%20Reference)))

(event EventTick
  (params (DeltaSeconds :type Float%20%28single-precision%29)))

(fn ConstructionScript)

(fn EquipItem
  (bind _returnvalue (Game|GetPlayerCharacter 0))
  (bind _statscomponent (Variables|Default|GetStatsComponent))
  (bind _astop_down_character (Utilities|Casting|CastToTopDownCharacter _returnvalue))
  (Variables|Default|SetisEquipped true)
  ;[1 0.8446 0] Add item stats to character's
  (Variables|/Game/TopDownCPP/Blueprints/TopDownCharacter.TopDownCharacter_C|SetStrength _astop_down_character (+ (Variables|/Game/TopDownCPP/Blueprints/TopDownCharacter.TopDownCharacter_C|GetStrength _astop_down_character) (Variables|/Game/Blueprints/StatsComponent.StatsComponent_C|GetStrength _statscomponent)))
  (Default|UpdateEndurance _astop_down_character (Variables|/Game/Blueprints/StatsComponent.StatsComponent_C|GetEndurance _statscomponent))
  (Variables|/Game/TopDownCPP/Blueprints/TopDownCharacter.TopDownCharacter_C|SetDexterity _astop_down_character (+ (Variables|/Game/TopDownCPP/Blueprints/TopDownCharacter.TopDownCharacter_C|GetDexterity _astop_down_character) (Variables|/Game/Blueprints/StatsComponent.StatsComponent_C|GetDexterity _statscomponent))))

(fn RemoveItem
  (bind _returnvalue (Game|GetPlayerCharacter 0))
  (bind _statscomponent (Variables|Default|GetStatsComponent))
  (bind _astop_down_character (Utilities|Casting|CastToTopDownCharacter _returnvalue))
  (Variables|Default|SetisEquipped false)
  ;[1 0.8446 0] Remove item stats to character's
  (Variables|/Game/TopDownCPP/Blueprints/TopDownCharacter.TopDownCharacter_C|SetStrength _astop_down_character (- (Variables|/Game/TopDownCPP/Blueprints/TopDownCharacter.TopDownCharacter_C|GetStrength _astop_down_character) (Variables|/Game/Blueprints/StatsComponent.StatsComponent_C|GetStrength _statscomponent)))
  (Default|UpdateEndurance _astop_down_character (* (Variables|/Game/Blueprints/StatsComponent.StatsComponent_C|GetEndurance _statscomponent) -1))
  (Variables|/Game/TopDownCPP/Blueprints/TopDownCharacter.TopDownCharacter_C|SetDexterity _astop_down_character (- (Variables|/Game/TopDownCPP/Blueprints/TopDownCharacter.TopDownCharacter_C|GetDexterity _astop_down_character) (Variables|/Game/Blueprints/StatsComponent.StatsComponent_C|GetDexterity _statscomponent))))